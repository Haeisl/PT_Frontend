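; Electrode grid actor that is placed on a patient's skin mesh and sends electrode positions to a server.
; Construction builds indicator meshes from rows, columns and cell size, marking corners with a separate material.
; While the move input is held, Tick snaps the grid to the skin under the cursor.
; SendElectrodePosition line-traces each point along the up vector onto the skin, then POSTs hits, center, corners and rotation as JSON.
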(event `self.ReceiveBeginPlay`
  (bind _asbp_game_mode_base (cast `/Game/Blueprints/GameMode/BP_GameModeBase` (`GameplayStatics.GetGameMode`))
    (:`then`
      (bind _output_get (set `self.PT Game Mode` _asbp_game_mode_base))
      (add `/Game/Blueprints/GameMode/BP_GameModeBase.GameModeInitReady` _output_get (delegate `GameModeReady`)))
    (:`CastFailed`
      (`KismetSystemLibrary.PrintString` "Casting failed"))))

(event `GameModeReady`
  (params (`Main User Interface` :type "/Game/Blueprints/UI/WBP_Main_UserInterface Object Reference"))
  (`self.Init` `Main User Interface`))

(event `self.ReceiveTick`
  (params (DeltaSeconds :type "Float (single-precision)"))
  (bind _hitresult (`PlayerController.GetHitResultUnderCursorByChannel` (`GameplayStatics.GetPlayerController` 0) "TraceTypeQuery1" true))
  (if (`|GetInputActionValue`)
    (if (== (`.HitActor` (`GameplayStatics.BreakHitResult` _hitresult)) (`/Game/Blueprints/3DData/BP_ConfigurationMeshActor.SkinMeshActor` (`self.BP_ConfigurationMeshActor`)))
      (`self.K2_SetActorLocationAndRotation` self (`.ImpactPoint` (`GameplayStatics.BreakHitResult` _hitresult)) (`KismetMathLibrary.Conv_VectorToRotator` (`.ImpactNormal` (`GameplayStatics.BreakHitResult` _hitresult))) false false)
      (`self.K2_AddActorLocalOffset` (5.0 0.0 0.0))
      (`self.K2_AddActorLocalRotation` self (struct :`Pitch` 90.0) false false)
      (else
        (`KismetSystemLibrary.PrintString` "NOT SKIN")))))

(fn `GenerateGrid`
  (params (InRowCount :type Integer) (InColumnCount :type Integer) (InCellSize :type "Float (double-precision)"))
  (bind _gridcornerrelative (`self.GridCornerRelative`))
  (bind _rows (`self.Rows`))
  (bind _columns (`self.Columns`))
  (bind _returnvalue (* _rows _columns))
  (set `self.Rows` InRowCount)
  (set `self.Columns` InColumnCount)
  (set `self.CellSize` InCellSize)
  (`self.ResetArrays`)
  (bind (_current_point _total_points _0_1_phase _poly_center) (`/Engine/ArtTools/RenderToTexture/Macros/RenderToTextureMacros.2D Grid Execution Macro` (`self.CellSize`) (0.0 0.0 0.0) _rows _columns)
    (:`Per Poly Execution`
      (bind _returnvalue_2 (`AddComponent|NODE_AddStaticMeshComponent-0` :`RelativeTransform` (`KismetMathLibrary.MakeTransform` _poly_center (struct) (0.01 0.01 0.01))))
      (if (== _current_point 0)
        (bind _output_get (set `self.GridCorner_A` _poly_center))
        (`PrimitiveComponent.SetMaterial` _returnvalue_2 0 "/Engine/MapTemplates/Materials/BasicAsset03.BasicAsset03" :!label _label)
        (`PrimitiveComponent.SetCastShadow` _returnvalue_2 true)
        (elif (== _current_point (- _rows 1))
          (bind _output_get_2 (set `self.GridCorner_B` _poly_center))
          (goto _label)
          (elif (== _current_point (- _returnvalue 1))
            (bind _output_get_3 (set `self.GridCorner_D` _poly_center))
            (goto _label)
            (elif (== _current_point (- _returnvalue _rows))
              (bind _output_get_4 (set `self.GridCorner_C` _poly_center))
              (goto _label)
              (else
                (`PrimitiveComponent.SetMaterial` _returnvalue_2 0 "/Engine/MapTemplates/Materials/BasicAsset01.BasicAsset01"))))))
      (`KismetArrayLibrary.Array_Add` (`self.Indicators`) _returnvalue_2)
      (`KismetArrayLibrary.Array_Add` (`self.RelativeRayStartPositions`) _poly_center)
      (`KismetArrayLibrary.Array_Add` (`self.ElectrodeNames`) (`KismetStringLibrary.Concat_StrStr` "Electrode_" (`KismetStringLibrary.Conv_IntToString` _current_point)))
      (`KismetArrayLibrary.Array_Add` _gridcornerrelative _output_get)
      (`KismetArrayLibrary.Array_Add` _gridcornerrelative _output_get_2)
      (`KismetArrayLibrary.Array_Add` _gridcornerrelative _output_get_4)
      (`KismetArrayLibrary.Array_Add` _gridcornerrelative _output_get_3))))

(fn `Init`
  (params (`Main User Interface` :type "/Game/Blueprints/UI/WBP_Main_UserInterface Object Reference"))
  (bind _returnvalue (`GameplayStatics.GetPlayerController` 0))
  (bind _returnvalue_2 (pcsubsystem `EnhancedInputLocalPlayerSubsystem` _returnvalue))
  (`/Engine/EditorBlueprintResources/StandardMacros.IsValid` `Main User Interface`
    (:`Is Valid`
      (bind _output_get (set `self.WBP User Interface` `Main User Interface`))
      (`self.EnableInput` _returnvalue)
      (`/Engine/EditorBlueprintResources/StandardMacros.IsValid` _returnvalue_2
        (:`Is Valid`
          (`EnhancedInputSubsystemInterface.AddMappingContext` _returnvalue_2 "/Game/Input/IMC_DefaultInput.IMC_DefaultInput" 0 (struct))
          (add `/Game/Blueprints/UI/WBP_Main_UserInterface.SendConfigurationData` _output_get (`|CreateDelegate` :!event `SendElectrodePosition`))
          (add `/Game/Blueprints/UI/WBP_Main_UserInterface.GridChanged` _output_get (`|CreateDelegate` :!event `GenerateGrid`)))
        (:`Is Not Valid`
          (`KismetSystemLibrary.PrintText` "Not Valid"))))
    (:`Is Not Valid`
      (`KismetSystemLibrary.PrintString` "Main User Interface Not Valid"))))

(fn `ResetArrays`
  (bind _indicators (`self.Indicators`))
  (for _array_element _indicators
    (`ActorComponent.K2_DestroyComponent` _array_element))
  (`KismetArrayLibrary.Array_Clear` _indicators)
  (`KismetArrayLibrary.Array_Clear` (`self.RelativeRayStartPositions`))
  (`KismetArrayLibrary.Array_Clear` (`self.ElectrodePositions`))
  (`KismetArrayLibrary.Array_Clear` (`self.ElectrodeNames`))
  (`KismetArrayLibrary.Array_Clear` (`self.GridCornerRelative`))
  (`KismetArrayLibrary.Array_Clear` (`self.GridCornerWorld`)))

(fn `SendElectrodePosition`
  (params (PatientID :type String) (ConfigID :type String))
  (bind _gridcornerworld (`self.GridCornerWorld`))
  (`self.ShootTracer`)
  (for _array_element (`self.GridCornerRelative`)
    (`KismetArrayLibrary.Array_Add` _gridcornerworld (`KismetMathLibrary.TransformLocation` (`self.GetTransform`) _array_element)))
  (bind _returnvalue (`self.CreateGridJSON` ConfigID PatientID (`self.ElectrodePositions`) (`self.ElectrodeNames`) (`self.CentralPoint`) (`self.CellSize`) _gridcornerworld (`self.GridRotation`) (`self.Rows`) (`self.Columns`)))
  (bind _returnvalue_2 (`PT_ConfigManager.GetElectrodesPositionAddress` PatientID ConfigID))
  (`PT_HTTPComponent.CallApiWithJSONBody` (`self.PT_HTTP_GRID_DATA`) _returnvalue_2 "POST" _returnvalue))

(fn `ShootTracer`
  (bind _bp_configurationmeshactor (`self.BP_ConfigurationMeshActor`))
  (bind _defaultsceneroot (`self.DefaultSceneRoot`))
  (bind _returnvalue (`KismetMathLibrary.TransformLocation` (`self.GetTransform`)))
  (bind _skinmeshactor (`/Game/Blueprints/3DData/BP_ConfigurationMeshActor.SkinMeshActor` _bp_configurationmeshactor))
  (bind _notskinmeshactor (`/Game/Blueprints/3DData/BP_ConfigurationMeshActor.NotSkinMeshActor` _bp_configurationmeshactor))
  (`KismetArrayLibrary.Array_Clear` (`self.ElectrodePositions`))
  (for _array_element (`self.RelativeRayStartPositions`)
    (bind _returnvalue_2 (`KismetMathLibrary.TransformLocation` (`self.GetTransform`) _array_element))
    (bind _outhit (`KismetSystemLibrary.LineTraceSingle` _returnvalue_2 (+ _returnvalue_2 (* (`SceneComponent.GetUpVector` _defaultsceneroot) (`self.Length`))) "TraceTypeQuery1" true _notskinmeshactor "ForDuration"))
    (if (== (`.HitActor` (`GameplayStatics.BreakHitResult` _outhit)) _skinmeshactor)
      (`KismetArrayLibrary.Array_Add` (`self.ElectrodePositions`) (`.ImpactPoint` (`GameplayStatics.BreakHitResult` _outhit)))
      (else
        (`KismetSystemLibrary.PrintString` "Not The Mesh Actor" :!label _label))))
  (bind _outhit_2 (`KismetSystemLibrary.LineTraceSingle` _returnvalue (+ _returnvalue (* (`SceneComponent.GetUpVector` _defaultsceneroot) (`self.Length`))) "TraceTypeQuery1" true _notskinmeshactor "ForDuration"))
  (if (== (`.HitActor` (`GameplayStatics.BreakHitResult` _outhit_2)) _skinmeshactor)
    (set `self.CentralPoint` (`.ImpactPoint` (`GameplayStatics.BreakHitResult` _outhit_2)))
    (set `self.GridRotation` (`self.K2_GetActorRotation`))
    (else
      (goto _label))))

(fn `UserConstructionScript`
  (`self.GenerateGrid` (`self.Rows`) (`self.Columns`) (`self.CellSize`)))
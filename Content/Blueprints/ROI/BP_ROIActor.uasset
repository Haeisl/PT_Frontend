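; BP_ROIActor is a region-of-interest actor that is edited through a configuration UI and saved per patient.
; Init binds the UI's position, length, rotation and send-data events and initializes the camera manager.
; HandleRoiChanged pushes current size, position and rotation back to the UI, while SendRoiData POSTs vertices and center as JSON over HTTP.
; BeginPlay hooks game-mode readiness; enhanced-input setup is disconnected, and IA_TriggerALT prints corner points.
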(event `self.ReceiveBeginPlay`
  (bind _asbp_game_mode_base (cast `/Game/Blueprints/GameMode/BP_GameModeBase` (`GameplayStatics.GetGameMode`))
    (:`then`
      (bind _output_get (set `self.PT_GameMode` _asbp_game_mode_base))
      (add `/Game/Blueprints/GameMode/BP_GameModeBase.GameModeInitReady` _output_get (`|CreateDelegate` :!event `Init`)))
    (:`CastFailed`
      (`KismetSystemLibrary.PrintString` "Casting failed"))))

(event `EnhancedInput|/Game/Input/IA_TriggerALT`
  (params (ActionValue :type Boolean) (ElapsedSeconds :type "Float (double-precision)") (TriggeredSeconds :type "Float (double-precision)") (InputAction :type "InputAction Object Reference" :default "/Game/Input/IA_TriggerALT.IA_TriggerALT"))
  (:`Triggered`
    (`self.PrintCornerPoints`)))

(event `TestEvent`
  (params (X :type "Float (double-precision)") (Y :type "Float (double-precision)") (Z :type "Float (double-precision)")))

(fn `HandleRoiChanged`
  (`/Game/Blueprints/UI/WBP_Main_UserInterface.UpdateRoiStats` (`self.ConfigurationUserInterface`) (`self.GetCurrentROISize`) (`self.GetCurrentROIPosition`) (`self.GetCurrentROIRotation`)))

(fn `Init`
  (params (`Main User Interface` :type "/Game/Blueprints/UI/WBP_Main_UserInterface Object Reference"))
  (bind _output_get (set `self.ConfigurationUserInterface` `Main User Interface`))
  (add `/Game/Blueprints/UI/WBP_Main_UserInterface.CommitPosition` _output_get (`|CreateDelegate` :!event `SetROIPosition`))
  (add `/Game/Blueprints/UI/WBP_Main_UserInterface.CommitLength` _output_get (`|CreateDelegate` :!event `SetROISize`))
  (add `/Game/Blueprints/UI/WBP_Main_UserInterface.CommitRotation` _output_get (`|CreateDelegate` :!event `SetROIRotation`))
  (add `/Game/Blueprints/UI/WBP_Main_UserInterface.SendRoiData` _output_get (`|CreateDelegate` :!event `SendRoiData`))
  (add `self.RoiChangedEvent` (`|CreateDelegate` :!event `HandleRoiChanged`))
  (`self.InitCurrentCameraManager`))

(fn `SendRoiData`
  (params (CurrentPatientID :type String) (CurrentROIID :type String))
  (bind _returnvalue (`PT_ConfigManager.GetRoiAddress` CurrentPatientID CurrentROIID))
  (bind _returnvalue_2 (`self.ConvertRoiToJson` CurrentPatientID CurrentROIID (`self.GetVertexArray`) (`self.GetCurrentROIPosition`)))
  (`PT_HTTPComponent.CallApiWithJSONBody` (`self.PT_HTTP_ROI_DATA`) _returnvalue "POST" _returnvalue_2))

(fn `UserConstructionScript`)
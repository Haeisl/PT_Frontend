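; Player-controlled camera actor on a spring arm that rotates, zooms and pans through Enhanced Input, with zoom blocked over relevant UI.
; A Tick-driven gate waits for the game mode's main UI, then fires camera init, which binds UI events for position reset and axis-aligned slicing views.
; Slicing toggle offsets a cube, but UpdateDissolveArea is empty: its dissolve parameter-collection logic is disconnected, as is Init's input-mapping setup.
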(event `self.ReceiveBeginPlay`
  (add `self.InitCamera` (`|CreateDelegate` :!event `Init`))
  (bind _asbp_game_mode_base (cast `/Game/Blueprints/GameMode/BP_GameModeBase` (`GameplayStatics.GetGameMode`))
    (:`then`
      (bind _output_get (set `self.PT_GameMode` _asbp_game_mode_base))
      (goto _label :!via `Open`))
    (:`CastFailed`
      (`KismetSystemLibrary.PrintString` "Casting failed"))))

(event `self.ReceiveTick`
  (params (DeltaSeconds :type "Float (single-precision)"))
  (`/Engine/EditorBlueprintResources/StandardMacros.Gate` true :!label _label
    (:`Exit`
      (`/Engine/EditorBlueprintResources/StandardMacros.IsValid` (`self.Main User Interface`)
        (:`Is Valid`
          _)
        (:`Is Not Valid`
          (bind _output_get (set `self.Main User Interface` (`/Game/Blueprints/GameMode/BP_GameModeBase.PT_MainUserInterface` (stale `self.ReceiveBeginPlay` _output_get))))
          (`/Engine/EditorBlueprintResources/StandardMacros.IsValid` _output_get
            (:`Is Valid`
              _))))
      (`self.InitCamera`)
      (goto _label :!via `Close`))))

(event `EnhancedInput|/Game/Input/IA_RotateCamera`
  (params (ActionValue :type "Vector2D Structure") (ElapsedSeconds :type "Float (double-precision)") (TriggeredSeconds :type "Float (double-precision)") (InputAction :type "InputAction Object Reference" :default "/Game/Input/IA_RotateCamera.IA_RotateCamera"))
  (bind _springarm (`self.SpringArm`))
  (:`Triggered`
    (`SceneComponent.K2_SetWorldRotation` _springarm (`KismetMathLibrary.MakeRotator` 0.0 (`KismetMathLibrary.FClamp` (+ (.pitch (.rotation (`SceneComponent.K2_GetComponentToWorld` _springarm))) (* ActionValue_Y 2.0)) -89.0 89.0) (+ (.yaw (.rotation (`SceneComponent.K2_GetComponentToWorld` _springarm))) (* ActionValue_X 2.0))) false false)
    (`self.UpdateDissolveArea`)))

(event `EnhancedInput|/Game/Input/IA_ZoomCamera`
  (params (ActionValue :type "Float (double-precision)") (ElapsedSeconds :type "Float (double-precision)") (TriggeredSeconds :type "Float (double-precision)") (InputAction :type "InputAction Object Reference" :default "/Game/Input/IA_ZoomCamera.IA_ZoomCamera"))
  (bind _camera (`self.Camera`))
  (bind (_relativelocation_x _relativelocation_y _relativelocation_z) (`KismetMathLibrary.BreakVector` (`SceneComponent.RelativeLocation` _camera)))
  (:`Triggered`
    (if (not (`/Game/Blueprints/UI/WBP_Main_UserInterface.IsMouseOverRelevantUI` (`self.Main User Interface`)))
      (`KismetSystemLibrary.MoveComponentTo` _camera (`KismetMathLibrary.MakeVector` (`KismetMathLibrary.FClamp` (+ _relativelocation_x (* ActionValue (`self.PT_CameraZoomSpeed`))) (`self.PT_MaxCameraDistance`) (`self.PT_MinCameraDistance`)) _relativelocation_y _relativelocation_z))
      (`self.UpdateDissolveArea`))))

(event `EnhancedInput|/Game/Input/IA_MoveCamera`
  (params (ActionValue :type "Vector2D Structure") (ElapsedSeconds :type "Float (double-precision)") (TriggeredSeconds :type "Float (double-precision)") (InputAction :type "InputAction Object Reference" :default "/Game/Input/IA_MoveCamera.IA_MoveCamera"))
  (bind _camera (`self.Camera`))
  (bind _pt_cameramovementspeed (`self.PT_CameraMovementSpeed`))
  (:`Triggered`
    (`self.K2_AddActorWorldOffset` (+ (* (`SceneComponent.GetRightVector` _camera) (* ActionValue_X _pt_cameramovementspeed)) (* (`SceneComponent.GetUpVector` _camera) (* ActionValue_Y _pt_cameramovementspeed))))))

(fn `Init`
  (bind _main_user_interface (`self.Main User Interface`))
  (add `/Game/Blueprints/UI/WBP_Main_UserInterface.ResetCameraPosition` _main_user_interface (`|CreateDelegate` :!event `ResetPosition`))
  (add `/Game/Blueprints/UI/WBP_Main_UserInterface.SetCameraForSlicing` _main_user_interface (`|CreateDelegate` :!event `SetCameraForSlicing`)))

(fn `ResetPosition`
  (`self.K2_SetActorLocationAndRotation` (0.0 0.0 0.0))
  (`self.UpdateDissolveArea`))

(fn `SetCameraForSlicing`
  (params (Axis :type "ESlicingType Enum" :default "X") (bIsInverted :type Boolean))
  (locals (RotationX :type "Rotator Structure" :default (struct)) (RotationXInverted :type "Rotator Structure" :default (struct :`Yaw` 180.0)) (RotationY :type "Rotator Structure" :default (struct :`Yaw` 90.0)) (RotationZ :type "Rotator Structure" :default (struct :`Pitch` 90.0 :`Yaw` 90.0)) (RotationZInverted :type "Rotator Structure" :default (struct :`Pitch` -90.0 :`Yaw` 90.0)))
  (bind _springarm (`self.SpringArm`))
  (bind _rotationy (`local.RotationY`))
  (switch `ESlicingType` Axis
    (:`X`
      (if bIsInverted
        (`SceneComponent.K2_SetWorldRotation` _springarm (`local.RotationXInverted`) false false)
        (else
          (`SceneComponent.K2_SetWorldRotation` _springarm (`local.RotationX`) false false))))
    (:`Y`
      (if bIsInverted
        (`SceneComponent.K2_SetWorldRotation` _springarm (`KismetMathLibrary.NegateRotator` _rotationy) false false)
        (else
          (`SceneComponent.K2_SetWorldRotation` _springarm _rotationy false false))))
    (:`Z`
      (if bIsInverted
        (`SceneComponent.K2_SetWorldRotation` _springarm (`local.RotationZInverted`) false false)
        (else
          (`SceneComponent.K2_SetWorldRotation` _springarm (`local.RotationZ`) false false))))))

(fn `ToggleCameraSlicing`
  (params (bIsCameraSlicing :type Boolean))
  (set `self.bIsSlicing` bIsCameraSlicing)
  (bind _result (`/Engine/EditorBlueprintResources/StandardMacros.NegateFloat` (`self.SlicingCubeOffset`))
    (:`  `
      (`SceneComponent.K2_AddLocalOffset` (`self.SlicingCube`) (`KismetMathLibrary.MakeVector` _result) false false)
      (`self.UpdateDissolveArea`))))

(fn `UpdateDissolveArea`)

(fn `UserConstructionScript`)
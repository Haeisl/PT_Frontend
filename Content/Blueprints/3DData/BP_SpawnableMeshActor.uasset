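; Spawnable actor that displays a procedural mesh built from supplied vertices, triangles, normals and vertex colors.
; The construction script creates the mesh section, enables collision only for material index 3, prints that index and applies the matching material from an array.
; UpdateMesh refreshes the section with new vertex colors, and SetVisbility toggles the mesh's visibility rather than setting it.
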(fn `Create Mesh`
  (bind _proceduralmesh (`self.ProceduralMesh`))
  (bind _materialindex (`self.MaterialIndex`))
  (`ProceduralMeshComponent.CreateMeshSection_LinearColor` :`self` _proceduralmesh :`Vertices` (`self.Vertices`) :`Triangles` (`self.Triangles`) :`Normals` (`self.Normals`) :`VertexColors` (`self.VertexColor`) :`bCreateCollision` (== _materialindex 3))
  (`KismetSystemLibrary.PrintString` (`KismetStringLibrary.Conv_IntToString` _materialindex))
  (`PrimitiveComponent.SetMaterial` _proceduralmesh 0 (`|GetArrayItem` (`self.Materials`) _materialindex)))

(fn `SetVisbility`
  (`SceneComponent.ToggleVisibility` (`self.ProceduralMesh`) false))

(fn `UpdateMesh`
  (params (VertexColors :type "Array of LinearColor Structure"))
  (`ProceduralMeshComponent.UpdateMeshSection_LinearColor` :`self` (`self.ProceduralMesh`) :`Vertices` (`self.Vertices`) :`Normals` (`self.Normals`) :`VertexColors` VertexColors))

(fn `UserConstructionScript`
  (`self.Create Mesh`))
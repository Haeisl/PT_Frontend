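; Actor that downloads a patient's configuration meshes over HTTP and displays them as separate 3D actors with UI visibility filters.
; RequestConfigurationMesh clears earlier arrays and requests compressed data; the HTTP callback parses the JSON into shared vertex and normal arrays plus per-mesh triangles.
; MeshDataLoaded spawns a BP_SpawnableMeshActor per mesh, separating the skin (description matches HitSurfaceName) from the rest, and registers each in the main UI's filter list.
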(event `self.ReceiveBeginPlay`
  (bind _asbp_game_mode_base (cast `/Game/Blueprints/GameMode/BP_GameModeBase` (`GameplayStatics.GetGameMode`))
    (:`then`
      (bind _output_get (set `self.PT_GameMode` _asbp_game_mode_base))
      (add `/Game/Blueprints/GameMode/BP_GameModeBase.GameModeInitReady` _output_get (`|CreateDelegate` :!event `Init`))
      (add `self.MeshDataLoadedCallbackEvent` (delegate `MeshDataLoaded`)))
    (:`CastFailed`
      (`KismetSystemLibrary.PrintString` "Casting failed"))))

(event `self.PT_HTTP_MESH.HttpCallbackEvent`
  (bind (_outvertexarray _outnormalarray _outmeshtagarray _outmeshdescriptionarray _outmeshdataarray) (`self.GetMultiMeshFromJSONResponseBody` (`self.PT_HTTP_MESH`))))

(event `MeshDataLoaded`
  (for (_array_element _array_index) (stale `self.PT_HTTP_MESH.HttpCallbackEvent` _outmeshdataarray)
    (bind _returnvalue (`|SpawnActorFromClass` "/Game/Blueprints/3DData/BP_SpawnableMeshActor.BP_SpawnableMeshActor_C" (`KismetMathLibrary.MakeTransform` (0.0 0.0 0.0)) "AlwaysSpawn" "OverrideRootScale" null (stale `self.PT_HTTP_MESH.HttpCallbackEvent` _outvertexarray) (stale `self.PT_HTTP_MESH.HttpCallbackEvent` _outnormalarray) (`.TriangleIndexArray` (break `PT_MeshData` _array_element)) (`self.GetVertexColorArray`) (break `PT_MeshData` _array_element) (`.Description` (break `PT_MeshData` _array_element)) _array_index null))
    (bind _returnvalue_2 (`KismetArrayLibrary.Array_Add` (`self.Meshes`) _returnvalue))
    (if (`KismetStringLibrary.EqualEqual_StrStr` (`.Description` (break `PT_MeshData` _array_element)) (`self.HitSurfaceName`))
      (set `self.SkinMeshActor` _returnvalue)
      (else
        (`KismetArrayLibrary.Array_Add` (`self.NotSkinMeshActor`) _returnvalue)))
    (`/Game/Blueprints/UI/WBP_Main_UserInterface.AddMeshFilterListItem` (`self.PT Main User Interface`) _returnvalue_2 (`KismetStringLibrary.Conv_StringToName` (`.Description` (break `PT_MeshData` _array_element))))))

(fn `Init`
  (params (PTMainUserInterface :type "/Game/Blueprints/UI/WBP_Main_UserInterface Object Reference"))
  (bind _output_get (set `self.PT Main User Interface` PTMainUserInterface))
  (add `/Game/Blueprints/UI/WBP_Main_UserInterface.SetVisibilityMesh` _output_get (`|CreateDelegate` :!event `Set Mesh Filter Visibility`))
  (add `/Game/Blueprints/UI/WBP_Main_UserInterface.LoadConfigurationData` _output_get (`|CreateDelegate` :!event `RequestConfigurationMesh`)))

(fn `RequestConfigurationMesh`
  (params (CurrentPatientID :type String))
  (`self.ResetSingle3DActorArrays`)
  (bind _returnvalue (`PT_ConfigManager.GetConfigurationMeshAddress` CurrentPatientID))
  (`PT_HTTPComponent.CallApiWithCompressedResponse` (`self.PT_HTTP_MESH`) _returnvalue "GET"))

(fn `Set Mesh Filter Visibility`
  (params (Index :type Integer))
  (`/Game/Blueprints/3DData/BP_SpawnableMeshActor.SetVisbility` (`|GetArrayItem` (`self.Meshes`) Index)))

(fn `UserConstructionScript`)
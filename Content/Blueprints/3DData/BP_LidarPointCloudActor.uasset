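; An actor that displays a Lidar point cloud built from stored point data and supports recoloring it at runtime.
; BeginPlay binds an update event and asynchronously creates the cloud from the data, then assigns it.
; UpdateLidarPointCloud applies a new color array to the data via stored vertex indices, then calls the update.
; The update event asynchronously rebuilds and reassigns the whole cloud, printing debug messages.
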(event `self.ReceiveBeginPlay`
  (add `self.UpdatePointCloud` (delegate `UpdatePointCloud_Event`))
  (bind (_progress _pointcloud) (`LidarPointCloudBlueprintLibrary.CreatePointCloudFromData` (`self.Point Cloud Data`) true)
    (:`Success`
      (bind _output_get (set `self.Point Cloud` _pointcloud))
      (`self.SetPointCloud` _output_get))
    (:`Failure`
      (`KismetSystemLibrary.PrintString` "Fail Lidar"))))

(event `UpdatePointCloud_Event`
  (`KismetSystemLibrary.PrintString` "Update....")
  (bind (_progress _pointcloud) (`LidarPointCloudBlueprintLibrary.CreatePointCloudFromData` (`self.Point Cloud Data`) true)
    (:`Success`
      (bind _output_get (set `self.Point Cloud` _pointcloud))
      (`self.SetPointCloud` _output_get)
      (`KismetSystemLibrary.PrintString` "New Point Cloud Set"))
    (:`Failure`
      (`KismetSystemLibrary.PrintString` "Fail Lidar"))))

(fn `UpdateLidarPointCloud`
  (params (NewColor :type "Array of LinearColor Structure"))
  (`KismetSystemLibrary.PrintString` "Create Lidar Point Cloud Data")
  (bind _outpointcloud (`self.UpdateLidarPointCloudColor` (`self.Point Cloud Data`) NewColor (`self.VertexIndicesArray`)))
  (set `self.Point Cloud Data` _outpointcloud)
  (`KismetSystemLibrary.PrintString` "FINISHED")
  (`self.UpdatePointCloud`))

(fn `UserConstructionScript`)
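; Actor that loads a patient's simulated 3D data over HTTP and displays it as mesh and point cloud actors.
; Parsed JSON becomes spawned actors registered in the main UI's filter lists, which toggle their visibility.
; After the first electrode fires, color updates use percentile bounds from the UI, respawning point clouds and updating meshes.
; Tick feeds mean magnitude of visible tags and mean normal-to-field angle to the UI.
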(event `self.ReceiveBeginPlay`
  (bind _asbp_game_mode_base (cast `/Game/Blueprints/GameMode/BP_GameModeBase` (`GameplayStatics.GetGameMode`))
    (:`then`
      (bind _output_get (set `self.PT_GameMode` _asbp_game_mode_base))
      (add `/Game/Blueprints/GameMode/BP_GameModeBase.GameModeInitReady` _output_get (`|CreateDelegate` :!event `Init`))
      (add `self.VolumeDataLoadedCallbackEvent` (delegate `VolumeDataLoadedCallbackEvent_Event`))
      (add `self.MeshDataLoadedCallbackEvent` (delegate `MeshDataLoadedCallbackEvent_Event`)))
    (:`CastFailed`
      (`KismetSystemLibrary.PrintString` "Casting failed"))))

(event `self.ReceiveTick`
  (params (DeltaSeconds :type "Float (single-precision)"))
  (`self.Update Mean`))

(event `self.PT_HTTP_3D_Data.HttpCallbackEvent`
  (bind _pt_http_3d_data (`self.PT_HTTP_3D_Data`))
  (bind (_outvertexarray _outvolumetagarray _outvolumedescriptionarray _outvolumedataarray) (`self.GetMultiVolumeFromJSONResponseBody` _pt_http_3d_data))
  (set `self.Volume Data Array` _outvolumedataarray)
  (`KismetSystemLibrary.PrintString` (`KismetStringLibrary.Conv_VectorToString` (`|GetArrayItem` _outvertexarray 9647)))
  (bind (_outvertexarray_2 _outnormalarray _outmeshtagarray _outmeshdescriptionarray _outmeshdataarray) (`self.GetMultiMeshFromJSONResponseBody` _pt_http_3d_data))
  (set `self.Mesh Data Array` _outmeshdataarray)
  (set `self.Normal Array` _outnormalarray))

(event `MeshDataLoadedCallbackEvent_Event`
  (for _array_element (stale `self.PT_HTTP_3D_Data.HttpCallbackEvent` _outmeshdataarray)
    (bind _returnvalue (`|SpawnActorFromClass` "/Game/Blueprints/3DData/BP_SpawnableMeshActor.BP_SpawnableMeshActor_C" (`KismetMathLibrary.MakeTransform` (0.0 0.0 0.0)) "AlwaysSpawn" "OverrideRootScale" null (stale `self.PT_HTTP_3D_Data.HttpCallbackEvent` _outvertexarray_2) (stale `self.PT_HTTP_3D_Data.HttpCallbackEvent` _outnormalarray) (`.TriangleIndexArray` (break `PT_MeshData` _array_element)) (`self.GetVertexColorArray`) (break `PT_MeshData` _array_element) (`.Description` (break `PT_MeshData` _array_element)) 9 null))
    (bind _returnvalue_2 (`KismetArrayLibrary.Array_Add` (`self.Meshes`) _returnvalue))
    (`/Game/Blueprints/UI/WBP_Main_UserInterface.AddMeshFilterListItem` (`self.PT Main User Interface`) _returnvalue_2 (`KismetStringLibrary.Conv_StringToName` (`KismetStringLibrary.Concat_StrStr` "Mesh " (`.Description` (break `PT_MeshData` _array_element)))))))

(event `VolumeDataLoadedCallbackEvent_Event`
  (for _array_element (stale `self.PT_HTTP_3D_Data.HttpCallbackEvent` _outvolumedataarray)
    (bind _returnvalue (`|SpawnActorFromClass` :`Class` "/Game/Blueprints/3DData/BP_LidarPointCloudActor.BP_LidarPointCloudActor_C" :`SpawnTransform` (`KismetMathLibrary.MakeTransform` (0.0 0.0 0.0)) :`CollisionHandlingOverride` "AlwaysSpawn" :`TransformScaleMethod` "MultiplyWithRoot" :`Point Cloud Data` (`.PointCloudArray` (break `PT_VolumeData` _array_element)) :`Instigator` null))
    (bind _returnvalue_2 (`KismetArrayLibrary.Array_Add` (`self.Volumes`) _returnvalue))
    (`/Game/Blueprints/UI/WBP_Main_UserInterface.AddVolumeFilterListItem` (`self.PT Main User Interface`) _returnvalue_2 (`KismetStringLibrary.Conv_StringToName` (`|GetArrayItem` (stale `self.PT_HTTP_3D_Data.HttpCallbackEvent` _outvolumedescriptionarray) _returnvalue_2)))))

(event `self.BP_Interpolation Actor.ElectrodeGridLoaded`
  (params (NumberOfElectrodes :type Integer)))

(event `self.BP_Interpolation Actor.BarycentricWeightsCalculated`
  (params (`Electrode A` :type Integer) (`Electrode B` :type Integer) (`Electrode C` :type Integer) (`Weight A` :type "Float (double-precision)") (`Weight B` :type "Float (double-precision)") (`Weight C` :type "Float (double-precision)")))

(fn `Init`
  (params (`Main User Interface` :type "/Game/Blueprints/UI/WBP_Main_UserInterface Object Reference"))
  (bind _output_get (set `self.PT Main User Interface` `Main User Interface`))
  (add `/Game/Blueprints/UI/WBP_Main_UserInterface.Load3DandData` _output_get (`|CreateDelegate` :!event `Load3DAndData`))
  (add `/Game/Blueprints/UI/WBP_Main_UserInterface.SetVisibilityVolume` _output_get (`|CreateDelegate` :!event `SetVisbilityVolume`))
  (add `/Game/Blueprints/UI/WBP_Main_UserInterface.UpdateColor` _output_get (`|CreateDelegate` :!event `UpdateColor`))
  (add `/Game/Blueprints/UI/WBP_Main_UserInterface.SetVisibilityMesh` _output_get (`|CreateDelegate` :!event `SetVisibilityMesh`))
  (add `/Game/Blueprints/UI/WBP_Main_UserInterface.PercentileSet` _output_get (`|CreateDelegate` :!event `SetPercentileForColor`)))

(fn `Load3DAndData`
  (params (PatientID :type String) (ConfigID :type String) (RoiID :type String))
  (`self.ResetMulti3DActorArrays`)
  (bind _returnvalue (`PT_ConfigManager.GetSimulated3DAddress` PatientID ConfigID))
  (`PT_HTTPComponent.CallApiWithCompressedResponse` (`self.PT_HTTP_3D_Data`) _returnvalue "GET"))

(fn `SetPercentileForColor`
  (params (Min :type "Float (double-precision)") (Max :type "Float (double-precision)"))
  (set `self.Min` Min)
  (set `self.Max` Max))

(fn `SetVisbilityVolume`
  (params (Index :type Integer))
  (bind _pointcloudcomponent (`LidarPointCloudActor.PointCloudComponent` (`|GetArrayItem` (`self.Volumes`) Index)))
  (bind _returnvalue (not (`SceneComponent.bVisible` _pointcloudcomponent)))
  (`KismetArrayLibrary.Array_Set` (`self.IsVolumeVisible`) Index _returnvalue)
  (`SceneComponent.SetVisibility` _pointcloudcomponent _returnvalue true))

(fn `SetVisibilityMesh`
  (params (Index :type Integer))
  (bind _ismeshvisible (`self.IsMeshVisible`))
  (if (not (== Index (`self.FilterIndexToIgnore`)))
    (`KismetArrayLibrary.Array_Set` _ismeshvisible Index (not (`|GetArrayItem` _ismeshvisible Index)))
    (`/Game/Blueprints/3DData/BP_SpawnableMeshActor.SetVisbility` (`|GetArrayItem` (`self.Meshes`) Index))))

(fn `Update Mean`
  (locals (MeanMagnitude :type "Float (double-precision)") (MeanVectorfield :type "Vector Structure") (Counter :type Integer) (Divider :type "Float (double-precision)" :default 1.0))
  (bind _pt_main_user_interface (`self.PT Main User Interface`))
  (bind _pt_simulation (`/Game/Blueprints/SimulationData/BP_InterpolationActor.PT_Simulation` (`self.BP_Interpolation Actor`)))
  (if (`/Game/Blueprints/SimulationData/BP_InterpolationActor.bIsFirstElectrodeFired` (`self.BP_Interpolation Actor`))
    (for (_array_element _array_index) (`self.IsVolumeVisible`)
      (if (or _array_element (`|GetArrayItem` (`self.IsMeshVisible`) _array_index))
        (bind (_outisvalid _returnvalue) (`PT_SimulationComponent.GetAverageMagnitudePerTag` _pt_simulation (+ _array_index 7)))
        (if _outisvalid
          (set `local.MeanMagnitude` (+ _returnvalue (`local.MeanMagnitude`)))
          (bind _result (`/Engine/EditorBlueprintResources/StandardMacros.IncrementInt` (`local.Counter`))
            (:`  `
              (set `local.Counter` _result))))))
    (if (== (`local.Counter`) 0)
      (`/Game/Blueprints/UI/WBP_Main_UserInterface.UpdateMetric` _pt_main_user_interface 0.0 (0.0 0.0 0.0))
      (else
        (`/Game/Blueprints/UI/WBP_Main_UserInterface.UpdateMetric` _pt_main_user_interface (* (`local.MeanMagnitude`) (/ (`local.Divider`) (`local.Counter`))) (0.0 0.0 0.0))))
    (bind _outmeanangle (`PT_SimulationComponent.CalculateMeanAngleBetweenNormalAndVectorField` _pt_simulation (`self.Normal Array`) (`PT_SimulationComponent.GetVectorfieldInRoi` _pt_simulation)))
    (`/Game/Blueprints/UI/WBP_Main_UserInterface.UpdateMetricGM` _pt_main_user_interface _outmeanangle)))

(fn `UpdateColor`
  (locals (NewPointClouds :type "Array of /Game/Blueprints/3DData/BP_LidarPointCloudActor Object Reference"))
  (bind _bp_interpolation_actor (`self.BP_Interpolation Actor`))
  (if (`/Game/Blueprints/SimulationData/BP_InterpolationActor.bIsFirstElectrodeFired` _bp_interpolation_actor)
    (bind (_outvertexcolor _inpercentileminvalue _inpercentilemaxvalue) (`/Game/Blueprints/SimulationData/BP_InterpolationActor.CalculateColor` _bp_interpolation_actor (`self.GetVertexArrayLength`) (`self.Min`) (`self.Max`)))
    (for (_array_element _array_index) (`self.Volumes`)
      (`self.K2_DestroyActor` _array_element)
      (bind (_id _vertexindexarray _pointcloudarray) (break `PT_VolumeData` (`|GetArrayItem` (`self.Volume Data Array`) _array_index)))
      (bind _outpointcloud (`self.UpdateLidarPointCloudColor` _pointcloudarray _outvertexcolor _vertexindexarray))
      (bind _returnvalue (`|SpawnActorFromClass` "/Game/Blueprints/3DData/BP_LidarPointCloudActor.BP_LidarPointCloudActor_C" (`KismetMathLibrary.MakeTransform` (0.0 0.0 0.0)) "AlwaysSpawn" "MultiplyWithRoot" null _outpointcloud _vertexindexarray null))
      (`KismetArrayLibrary.Array_Add` (`local.NewPointClouds`) _returnvalue)
      (`SceneComponent.SetVisibility` (`Actor.RootComponent` _returnvalue) (`|GetArrayItem` (`self.IsVolumeVisible`) _array_index) true)
      (`/Game/Blueprints/UI/WBP_Main_UserInterface.Update Min Max Color Percentile Values` (`self.PT Main User Interface`) _inpercentileminvalue _inpercentilemaxvalue))
    (`KismetArrayLibrary.Array_Clear` (`self.Volumes`))
    (set `self.Volumes` (`local.NewPointClouds`))
    (for _array_element_2 (`self.Meshes`)
      (`/Game/Blueprints/3DData/BP_SpawnableMeshActor.UpdateMesh` _array_element_2 _outvertexcolor))))

(fn `UserConstructionScript`)
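; BP_SkinMeshActor fetches a patient's skin mesh over HTTP and displays it as a procedural mesh.
; Init binds it to the main UI's 3D-load and mesh-visibility events, and LoadSkinMesh sends a GET request by patient ID.
; The HTTP callback converts the JSON into a collidable mesh section with a dissolve-area material, adds a "Skin" filter entry, and signals readiness.
; Selecting the matching filter index toggles the mesh's visibility.
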(event `self.ReceiveBeginPlay`
  (bind _asbp_game_mode_base (cast `/Game/Blueprints/GameMode/BP_GameModeBase` (`GameplayStatics.GetGameMode`))
    (:`then`
      (bind _output_get (set `self.PT Game Mode` _asbp_game_mode_base))
      (add `/Game/Blueprints/GameMode/BP_GameModeBase.GameModeInitReady` _output_get (`|CreateDelegate` :!event `Init`)))
    (:`CastFailed`
      (`KismetSystemLibrary.PrintString` "Casting failed"))))

(event `self.PT_HTTP_SKIN_MESH.HttpCallbackEvent`
  (bind (_outvertexarray _outtriangleindexarray _outnormalarray) (`self.ConvertJSONResponseBodyToMesh` (`self.PT_HTTP_SKIN_MESH`)))
  (`ProceduralMeshComponent.CreateMeshSection_LinearColor` :`self` (`self.ProceduralMesh`) :`Vertices` _outvertexarray :`Triangles` _outtriangleindexarray :`Normals` _outnormalarray :`bCreateCollision` true)
  (`PrimitiveComponent.SetMaterial` (`self.ProceduralMesh`) 0 "/Game/Materials/SlicingMaterials/M_PT_DissolveArea_Inst.M_PT_DissolveArea_Inst")
  (`/Game/Blueprints/UI/WBP_Main_UserInterface.AddMeshFilterListItem` (`self.Main User Interface`) (`self.FilterIndex`) "Skin")
  (`self.SkinMeshReady`))

(fn `Init`
  (params (`Main User Interface` :type "/Game/Blueprints/UI/WBP_Main_UserInterface Object Reference"))
  (bind _output_get (set `self.Main User Interface` `Main User Interface`))
  (add `/Game/Blueprints/UI/WBP_Main_UserInterface.Load3DandData` _output_get (`|CreateDelegate` :!event `LoadSkinMesh`))
  (add `/Game/Blueprints/UI/WBP_Main_UserInterface.SetVisibilityMesh` _output_get (`|CreateDelegate` :!event `SetMeshFilterFisibility`)))

(fn `LoadSkinMesh`
  (params (PatientID :type String) (ConfigID :type String) (RoiID :type String))
  (bind _returnvalue (`PT_ConfigManager.GetSkinMeshAddress` PatientID))
  (`PT_HTTPComponent.CallApi` (`self.PT_HTTP_SKIN_MESH`) _returnvalue "GET"))

(fn `SetMeshFilterFisibility`
  (params (Index :type Integer))
  (if (== Index (`self.FilterIndex`))
    (`SceneComponent.ToggleVisibility` (`self.ProceduralMesh`) false)))

(fn `UserConstructionScript`)
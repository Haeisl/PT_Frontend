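; Interactive actor that lets the user move an electrode over a patient's skin mesh and interpolates pre-simulated field data for that position.
; HTTP calls load the electrode area, validation and simulation data, building an indicator grid over an invisible procedural quad.
; Cursor hits on the quad are traced onto the skin, yielding barycentric weights from three nearest grid electrodes.
; PTSimulation blends their data for UI metrics, percentile-based vertex colours and JSON upload.
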(event `self.ReceiveBeginPlay`
  (bind _asbp_game_mode_base (cast `/Game/Blueprints/GameMode/BP_GameModeBase` (`GameplayStatics.GetGameMode`))
    (:`then`
      (bind _output_get (set `self.PT Game Mode` _asbp_game_mode_base))
      (add `/Game/Blueprints/GameMode/BP_GameModeBase.GameModeInitReady` _output_get (`|CreateDelegate` :!event `Init`)))
    (:`CastFailed`
      (`KismetSystemLibrary.PrintString` "Casting failed"))))

(event `self.ReceiveTick`
  (params (DeltaSeconds :type "Float (single-precision)"))
  (`self.HandleElectrodeMovement`))

(event `self.PT_HTTP_INTERPOLATION_AREA.HttpCallbackEvent`
  (`self.HandleHttpCallback`)
  (bind _returnvalue (`PT_ConfigManager.GetDataVallidationAddress` (`self.Patient ID`) (`self.Config ID`)))
  (`PT_HTTPComponent.CallApi` (`self.PT_HTTP_VALIDATION_DATA`) _returnvalue "GET"))

(event `self.PT_HTTP_VALIDATION_DATA.HttpCallbackEvent`
  (bind _corruptedelectrodes (`self.CorruptedElectrodes`))
  (bind (_outelectrodecount _outsuccessfullelectrodeindex _outiscorrupted) (`self.ProcessValidationResponseData` (`self.PT_HTTP_VALIDATION_DATA`)))
  (bind _output_get (set `self.Out Successfull Electrode Index` _outsuccessfullelectrodeindex))
  (`KismetArrayLibrary.Array_Resize` _corruptedelectrodes _outelectrodecount)
  (for _array_element _output_get
    (`KismetArrayLibrary.Array_Set` _corruptedelectrodes _array_element true)
    (`PrimitiveComponent.SetMaterial` (`|GetArrayItem` (`self.Indicators`) _array_element) 0 "/Engine/MapTemplates/Materials/BasicAsset03.BasicAsset03"))
  (for _array_element_2 (`self.Indicators`)
    (`PrimitiveComponent.SetCastShadow` _array_element_2 false))
  (if _outiscorrupted
    (`/Game/Blueprints/UI/WBP_Main_UserInterface.Trigger Notification Message` (`self.PT Main User Interface`) "CautionHeadline" "ErrorMessageFailedSimulationInConfig")))

(event `self.PT_HTTP_SIMULATION_DATA.HttpCallbackEvent`
  (`PT_SimulationComponent.GetSimulationDataFromJSONResponseBody` (`self.PT_Simulation`) (`self.PT_HTTP_SIMULATION_DATA`) (`PT_ConfigManager.GetDataTagArray`) (`self.NumberOfPreSimulatedElectrodes`))
  (set `self.bIsSimulationDataLoaded` true)
  (if (`self.bIsSkinMeshReady`)
    (`self.FireFirstElectrode` :!label _label)))

(event `self.BP_SkinMeshActor.SkinMeshReady`
  (set `self.bIsSkinMeshReady` true)
  (if (`self.bIsSimulationDataLoaded`)
    (goto _label)))

(fn `CalculateColor`
  (params (InVertexArrayLength :type Integer) (InPercentileMin :type "Float (double-precision)") (InPercentileMax :type "Float (double-precision)"))
  (returns (OutVertexColor :type "Array of LinearColor Structure") (InPercentileMinValue :type "Float (double-precision)") (InPercentileMaxValue :type "Float (double-precision)"))
  (bind _pt_simulation (`self.PT_Simulation`))
  (bind _pt_simulation_2 (`self.PT_Simulation`))
  (bind _returnvalue (`PT_SimulationComponent.CalculatePercentileForInterpolatedMagnitudeDataPerTagArray` _pt_simulation_2 InPercentileMin))
  (bind _returnvalue_2 (`PT_SimulationComponent.CalculatePercentileForInterpolatedMagnitudeDataPerTagArray` _pt_simulation_2 InPercentileMax))
  (for _array_element (`PT_ConfigManager.GetDataTagIndexArray`)
    (bind _asbp_my_game_instance (cast `/Game/Blueprints/GameInstance/BP_MyGameInstance` (`GameplayStatics.GetGameInstance`)))
    (bind _returnvalue_3 (`PT_SimulationComponent.GetInterpolatedMagnitudeDataPerTag` _pt_simulation _array_element))
    (`PT_MyGameInstance.SetInterpolatedData` _asbp_my_game_instance _returnvalue_3)
    (bind _foundwidgets (`WidgetBlueprintLibrary.GetAllWidgetsOfClass` "/Game/Blueprints/UI/WBP_MetricManager.WBP_MetricManager_C" false))
    (if (`/Game/Blueprints/UI/WBP_MetricManager.IsGrayscale` (`|GetArrayItem` _foundwidgets))
      (bind _returnvalue_4 (`PT_SimulationComponent.MapToGreyscaleColormap` _pt_simulation _returnvalue_3 _array_element _returnvalue _returnvalue_2))
      (`PT_SimulationComponent.SetDataColorArrayPerTag` _pt_simulation _array_element _returnvalue_4)
      (else
        (bind _returnvalue_5 (`PT_SimulationComponent.MapToPlasmaColormap` _pt_simulation _returnvalue_3 _array_element _returnvalue _returnvalue_2))
        (`PT_SimulationComponent.SetDataColorArrayPerTag` _pt_simulation _array_element _returnvalue_5))))
  (bind _returnvalue_6 (`PT_SimulationComponent.CalculateVertexColors` _pt_simulation InVertexArrayLength))
  (return _returnvalue_6 _returnvalue _returnvalue_2))

(fn `FireFirstElectrode`
  (bind (_firstelectrodeposition_x _firstelectrodeposition_y) (`KismetMathLibrary.BreakVector` (`self.FirstElectrodePosition`)))
  (bind _world_location (`self.TransformToWorldSpace` (`KismetMathLibrary.MakeVector` _firstelectrodeposition_x _firstelectrodeposition_y (`self.bFirstElectrodeTraceDistance`))))
  (if (not (`self.bIsFirstElectrodeFired`))
    (set `self.bIsFirstElectrodeFired` true)
    (bind _outhit (`KismetSystemLibrary.LineTraceSingle` :`Start` _world_location :`End` (+ _world_location (* (`SceneComponent.GetUpVector` (`self.DefaultSceneRoot`)) (`self.Length`))) :`TraceChannel` "TraceTypeQuery1" :`bTraceComplex` true :`bIgnoreSelf` false :`DrawTime` 1.0))
    (`KismetSystemLibrary.PrintString` (`KismetStringLibrary.Conv_BoolToString` (`GameplayStatics.BreakHitResult` _outhit)))
    (if (== (`self.ProceduralMesh`) (`.HitComponent` (`GameplayStatics.BreakHitResult` _outhit)))
      (`KismetSystemLibrary.PrintString` (`KismetStringLibrary.Conv_VectorToString` (`.ImpactPoint` (`GameplayStatics.BreakHitResult` _outhit))))
      (`SceneComponent.K2_SetWorldLocationAndRotation` (`self.Electrode`) (`.ImpactPoint` (`GameplayStatics.BreakHitResult` _outhit)) (`KismetMathLibrary.MakeRotFromZ` (`.ImpactNormal` (`GameplayStatics.BreakHitResult` _outhit))) false false)
      (`self.HandleElectrode` (`.ImpactPoint` (`GameplayStatics.BreakHitResult` _outhit))))))

(fn `GenerateGrid`
  (params (GridSpacing :type "Float (double-precision)") (Rows :type Integer) (Columns :type Integer))
  (bind (_current_point _total_points _0_1_phase _poly_center) (`/Engine/ArtTools/RenderToTexture/Macros/RenderToTextureMacros.2D Grid Execution Macro` GridSpacing (0.0 0.0 0.0) Rows Columns)
    (:`Per Poly Execution`
      (bind _returnvalue (`AddComponent|NODE_AddStaticMeshComponent-0` :`RelativeTransform` (`KismetMathLibrary.MakeTransform` _poly_center (struct) (0.01 0.01 0.01))))
      (`KismetArrayLibrary.Array_Add` (`self.Indicators`) _returnvalue)
      (bind _returnvalue_2 (`AddComponent|NODE_AddStaticMeshComponent-5` :`RelativeTransform` (`KismetMathLibrary.MakeTransform` _poly_center (struct) (`self.Indicator Scale`))))
      (`SceneComponent.SetVisibility` _returnvalue_2 false false)
      (`KismetArrayLibrary.Array_Add` (`self.IndicatorsActive`) _returnvalue_2)
      (`KismetArrayLibrary.Array_Add` (`self.RelativeRayStartPosition`) _poly_center)
      (`KismetArrayLibrary.Array_Add` (`self.ElectrodeNames`) (`KismetStringLibrary.Concat_StrStr` "Electrode_" (`KismetStringLibrary.Conv_IntToString` _current_point))))))

(fn `HandleBarycentricSimulation`
  (params (`Electrode A` :type Integer) (`Electrode B` :type Integer) (`Electrode C` :type Integer) (`Weight A` :type "Float (double-precision)") (`Weight B` :type "Float (double-precision)") (`Weight C` :type "Float (double-precision)"))
  (bind _pt_simulation (`self.PT_Simulation`))
  (`PT_SimulationComponent.ProcessInterpolation` _pt_simulation `Electrode A` `Electrode B` `Electrode C` `Weight A` `Weight B` `Weight C`)
  (`/Game/Blueprints/UI/WBP_Main_UserInterface.UpdateMetric` (`self.PT Main User Interface`) (`PT_SimulationComponent.GetAverageMagnitude` _pt_simulation) (`PT_SimulationComponent.GetAverageVectorField` _pt_simulation)))

(fn `HandleElectrode`
  (params (StartPosition :type "Vector Structure"))
  (locals (IndicatorScale :type "Vector Structure" :default (0.01 0.01 0.02)))
  (bind _locallocation (`self.TransformToLocalSpace` StartPosition))
  (bind _presimulatedelectrodepositions (`self.PreSimulatedElectrodePositions`))
  (bind _corruptedelectrodes (`self.CorruptedElectrodes`))
  (bind _outhit (`KismetSystemLibrary.LineTraceSingle` :`Start` StartPosition :`End` (+ StartPosition (* (`SceneComponent.GetUpVector` (`self.DefaultSceneRoot`)) (`self.Length`))) :`TraceChannel` "TraceTypeQuery1" :`bTraceComplex` true :`DrawTime` 1.0))
  (if (== (`.HitActor` (`GameplayStatics.BreakHitResult` _outhit)) (`self.BP_SkinMeshActor`))
    (bind _output_get (set `self.CurrentElectrodePosition` (`.ImpactPoint` (`GameplayStatics.BreakHitResult` _outhit))))
    (bind _outnearestneighborsgridindicies (`self.FindNearestNeighbors` (`KismetMathLibrary.MakeVector` (.x _locallocation) (.y _locallocation)) (`self.RelativeRayStartPosition`)))
    (bind _output (`|GetArrayItem` _outnearestneighborsgridindicies))
    (bind _output_2 (`|GetArrayItem` _presimulatedelectrodepositions _output))
    (bind _output_3 (`|GetArrayItem` _outnearestneighborsgridindicies 1))
    (bind _output_4 (`|GetArrayItem` _presimulatedelectrodepositions _output_3))
    (bind _output_5 (`|GetArrayItem` _outnearestneighborsgridindicies 2))
    (bind _output_6 (`|GetArrayItem` _presimulatedelectrodepositions _output_5))
    (bind (_outweighta _outweightb _outweightc) (`self.BarycentricWeightCalculation` _output_get _output_2 _output_4 _output_6))
    (`/Game/Blueprints/UI/WBP_Main_UserInterface.UpdateElectrodePosition` (`self.PT Main User Interface`) _output_get)
    (`self.BarycentricWeightsCalculated` _output _output_3 _output_5 _outweighta _outweightb _outweightc)
    (`/Game/Blueprints/UI/WBP_Main_UserInterface.UpdateInterpolationElectrodes` (`self.PT Main User Interface`) _output _output_3 _output_5 (`self.TransformToLocalSpace` _output_2) (`self.TransformToLocalSpace` _output_4) (`self.TransformToLocalSpace` _output_6) (not (`|GetArrayItem` _corruptedelectrodes _output)) (not (`|GetArrayItem` _corruptedelectrodes _output_3)) (not (`|GetArrayItem` _corruptedelectrodes _output_5)) _locallocation)
    (`self.ToggleActiveIndicators` _output _output_3 _output_5)
    (else
      (`KismetSystemLibrary.PrintString` "Not The Skin"))))

(fn `HandleElectrodeMovement`
  (bind _hitresult (`PlayerController.GetHitResultUnderCursorByChannel` (`GameplayStatics.GetPlayerController` 0) "TraceTypeQuery1" true))
  (if (`|GetInputActionValue`)
    (if (== (`self.ProceduralMesh`) (`.HitComponent` (`GameplayStatics.BreakHitResult` _hitresult)))
      (if (!= (stale _output_get) (`.ImpactPoint` (`GameplayStatics.BreakHitResult` _hitresult)))
        (bind _output_get (set `self.oldElectrodePosition` (`.ImpactPoint` (`GameplayStatics.BreakHitResult` _hitresult))))
        (`SceneComponent.K2_SetWorldLocationAndRotation` (`self.Electrode`) (`.ImpactPoint` (`GameplayStatics.BreakHitResult` _hitresult)) (`KismetMathLibrary.MakeRotFromZ` (`.ImpactNormal` (`GameplayStatics.BreakHitResult` _hitresult))) false false)
        (`self.HandleElectrode` (`.ImpactPoint` (`GameplayStatics.BreakHitResult` _hitresult)))))))

(fn `HandleHttpCallback`
  (bind _vertices (`self.Vertices`))
  (bind _proceduralmesh (`self.ProceduralMesh`))
  (`self.ResetArray`)
  (bind (_outcenter _outa _outb _outc _outd _outrotation _outrows _outcolumns _outcellsize _outnumber _outelectrodepositions) (`self.ProcessResponseData` (`self.PT_HTTP_INTERPOLATION_AREA`)))
  (set `self.PreSimulatedElectrodePositions` _outelectrodepositions)
  (bind _output_get (set `self.Rows` _outrows))
  (bind _output_get_2 (set `self.Columns` _outcolumns))
  (bind _output_get_3 (set `self.GridSpacing` _outcellsize))
  (bind _output_get_4 (set `self.NumberOfPreSimulatedElectrodes` _outnumber))
  (`self.K2_SetActorLocationAndRotation` _outcenter _outrotation)
  (`self.GenerateGrid` _output_get_3 _output_get _output_get_2)
  (`KismetArrayLibrary.Array_Add` _vertices (* (`self.TransformToLocalSpace` _outa) (1.0 1.0 0.0)))
  (`KismetArrayLibrary.Array_Add` _vertices (* (`self.TransformToLocalSpace` _outb) (1.0 1.0 0.0)))
  (`KismetArrayLibrary.Array_Add` _vertices (* (`self.TransformToLocalSpace` _outc) (1.0 1.0 0.0)))
  (`KismetArrayLibrary.Array_Add` _vertices (* (`self.TransformToLocalSpace` _outd) (1.0 1.0 0.0)))
  (bind _triangles (`KismetProceduralMeshLibrary.CreateGridMeshTriangles` 2 2))
  (bind _output_get_5 (set `self.Triangles` _triangles))
  (`ProceduralMeshComponent.CreateMeshSection_LinearColor` :`self` _proceduralmesh :`Vertices` (`self.Vertices`) :`Triangles` _output_get_5 :`bCreateCollision` true)
  (`PrimitiveComponent.CreateDynamicMaterialInstance` _proceduralmesh 0 "/Engine/VREditor/UI/ArrowMaterial.ArrowMaterial" "None")
  (`SceneComponent.SetVisibility` _proceduralmesh false false)
  (`self.ElectrodeGridLoaded` _output_get_4))

(fn `Init`
  (params (`Main User Interface` :type "/Game/Blueprints/UI/WBP_Main_UserInterface Object Reference"))
  (bind _returnvalue (`GameplayStatics.GetPlayerController` 0))
  (bind _returnvalue_2 (pcsubsystem `EnhancedInputLocalPlayerSubsystem` _returnvalue))
  (`self.EnableInput` _returnvalue)
  (`/Engine/EditorBlueprintResources/StandardMacros.IsValid` _returnvalue_2
    (:`Is Valid`
      (`EnhancedInputSubsystemInterface.AddMappingContext` _returnvalue_2 "/Game/Input/IMC_DefaultInput.IMC_DefaultInput" 0 (struct))
      (bind _output_get (set `self.PT Main User Interface` `Main User Interface`))
      (add `/Game/Blueprints/UI/WBP_Main_UserInterface.Load3DandData` _output_get (`|CreateDelegate` :!event `LoadElectrodeArea`))
      (add `/Game/Blueprints/UI/WBP_Main_UserInterface.Load3DandData` _output_get (`|CreateDelegate` :!event `LoadSimulationData`))
      (add `/Game/Blueprints/UI/WBP_Main_UserInterface.SendInterpolationData` _output_get (`|CreateDelegate` :!event `SendInterpolationData`))
      (add `self.BarycentricWeightsCalculated` (`|CreateDelegate` :!event `HandleBarycentricSimulation`))
      (add `/Game/Blueprints/UI/WBP_Main_UserInterface.SetInterpolationElectrode` _output_get (`|CreateDelegate` :!event `SetElectrodePosition`))
      (add `/Game/Blueprints/UI/WBP_Main_UserInterface.SetVisibilityVolume` _output_get (`|CreateDelegate` :!event `SetUsedTag`))
      (add `/Game/Blueprints/UI/WBP_Main_UserInterface.SetVisibilityMesh` _output_get (`|CreateDelegate` :!event `SetUsedTag`)))
    (:`Is Not Valid`
      (`KismetSystemLibrary.PrintText` "Not Valid"))))

(fn `LoadElectrodeArea`
  (params (PatientID :type String) (ConfigID :type String) (RoiID :type String))
  (`self.ResetArray`)
  (bind _output_get (set `self.Patient ID` PatientID))
  (bind _output_get_2 (set `self.Config ID` ConfigID))
  (bind _returnvalue (`PT_ConfigManager.GetElectrodesPositionAddress` _output_get _output_get_2))
  (`PT_HTTPComponent.CallApi` (`self.PT_HTTP_INTERPOLATION_AREA`) _returnvalue "GET"))

(fn `LoadSimulationData`
  (params (PatientID :type String) (ConfigID :type String) (RoiID :type String))
  (`PT_SimulationComponent.ResetSimulationDataArrays` (`self.PT_Simulation`))
  (bind _returnvalue (`PT_ConfigManager.GetSimulatedDataAddress` PatientID ConfigID RoiID))
  (`PT_HTTPComponent.CallApiWithCompressedResponse` (`self.PT_HTTP_SIMULATION_DATA`) _returnvalue "GET"))

(fn `ResetArray`
  (bind _indicators (`self.Indicators`))
  (for _array_element _indicators
    (`ActorComponent.K2_DestroyComponent` _array_element))
  (`KismetArrayLibrary.Array_Clear` _indicators)
  (`KismetArrayLibrary.Array_Clear` (`self.Vertices`))
  (`KismetArrayLibrary.Array_Clear` (`self.Triangles`))
  (`KismetArrayLibrary.Array_Clear` (`self.ElectrodeNames`))
  (`KismetArrayLibrary.Array_Clear` (`self.PreSimulatedElectrodePositions`))
  (`KismetArrayLibrary.Array_Clear` (`self.RelativeRayStartPosition`)))

(fn `SendInterpolationData`
  (params (PatientID :type String) (ConfigID :type String) (RoiID :type String) (InterpolationID :type String))
  (bind _outjsonstring (`PT_SimulationComponent.CreateInterpolatedDataJson` (`self.PT_Simulation`) PatientID ConfigID RoiID InterpolationID (`self.CurrentElectrodePosition`) (`self.GridSpacing`)))
  (bind _returnvalue (`PT_ConfigManager.GetInterpolatedDataAddress` PatientID ConfigID RoiID InterpolationID))
  (`PT_HTTPComponent.CallApiWithJSONBody` (`self.PT_HTTP_INTERPOLATED_DATA`) _returnvalue "POST" _outjsonstring))

(fn `SetElectrodePosition`
  (params (X :type "Float (double-precision)") (Y :type "Float (double-precision)"))
  (bind _electrode (`self.Electrode`))
  (bind (_relativelocation_x _relativelocation_y _relativelocation_z) (`KismetMathLibrary.BreakVector` (`SceneComponent.RelativeLocation` _electrode)))
  (bind _output_get (set `self.oldElectrodePosition` (`KismetMathLibrary.MakeVector` X Y _relativelocation_z)))
  (bind _world_location (`self.TransformToWorldSpace` _output_get))
  (`SceneComponent.K2_SetWorldLocation` _electrode _world_location false false)
  (`self.HandleElectrode` _world_location))

(fn `SetUsedTag`
  (params (Index :type Integer)))

(fn `ToggleActiveIndicators`
  (params (IndexA :type "Integer (by ref)") (IndexB :type "Integer (by ref)") (IndexC :type "Integer (by ref)"))
  (bind _indicatorsactive (`self.IndicatorsActive`))
  (for _array_element _indicatorsactive
    (`SceneComponent.SetVisibility` _array_element false false))
  (`SceneComponent.SetVisibility` (`|GetArrayItem` _indicatorsactive IndexA) true false)
  (`SceneComponent.SetVisibility` (`|GetArrayItem` _indicatorsactive IndexB) true false)
  (`SceneComponent.SetVisibility` (`|GetArrayItem` _indicatorsactive IndexC) true false)
  (return))

(fn `TransformToLocalSpace`
  (params (WorldLocation :type "Vector Structure"))
  (returns (LocalLocation :type "Vector Structure"))
  (return (`KismetMathLibrary.InverseTransformLocation` (`self.GetTransform`) WorldLocation)))

(fn `TransformToWorldSpace`
  (params (`Local Location` :type "Vector Structure"))
  (returns (`World Location` :type "Vector Structure"))
  (return (`KismetMathLibrary.TransformLocation` (`self.GetTransform`) `Local Location`)))

(fn `UserConstructionScript`)
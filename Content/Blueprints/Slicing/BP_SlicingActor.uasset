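; Slicing actor for one X, Y or Z axis that drives a dissolve-based cutting volume through its SlicingCube.
; It hooks into game mode readiness, and Init binds main UI events for updating, inverting, resetting and switching slicing view.
; Handlers move or flip the cube along its axis, or park the actor during camera slicing.
; Each change writes the cube's world location and scale to MPC_DissolveArea for materials to read.
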(event `self.ReceiveBeginPlay`
  (bind _asbp_game_mode_base (cast `/Game/Blueprints/GameMode/BP_GameModeBase` (`GameplayStatics.GetGameMode`))
    (:`then`
      (bind _output_get (set `self.PT_GameMode` _asbp_game_mode_base))
      (add `/Game/Blueprints/GameMode/BP_GameModeBase.GameModeInitReady` _output_get (`|CreateDelegate` :!event `Init`)))
    (:`CastFailed`
      (`KismetSystemLibrary.PrintString` "Casting failed"))))

(fn `Init`
  (params (`Main User Interface` :type "/Game/Blueprints/UI/WBP_Main_UserInterface Object Reference"))
  (bind _output_get (set `self.PT Main User Interface` `Main User Interface`))
  (add `/Game/Blueprints/UI/WBP_Main_UserInterface.InvertSlicing` _output_get (`|CreateDelegate` :!event `ToogleInvertSlicing`))
  (add `/Game/Blueprints/UI/WBP_Main_UserInterface.ResetSlicing` _output_get (`|CreateDelegate` :!event `Reset`))
  (add `/Game/Blueprints/UI/WBP_Main_UserInterface.SwitchSlicingView` _output_get (`|CreateDelegate` :!event `ToogleActiveSlicing`))
  (add `/Game/Blueprints/UI/WBP_Main_UserInterface.UpdateSlicing` _output_get (`|CreateDelegate` :!event `MoveSlicingCube`)))

(fn `MoveSlicingCube`
  (params (SlicingOffset :type "Float (double-precision)") (SicingType :type "ESlicingType Enum" :default "X"))
  (bind _slicingtype (`self.SlicingType`))
  (bind _slicingcube (`self.SlicingCube`))
  (bind _inverted (`self.Inverted`))
  (bind _returnvalue (`KismetMathLibrary.Conv_VectorToLinearColor` (`SceneComponent.K2_GetComponentLocation` _slicingcube)))
  (bind _returnvalue_2 (`KismetMathLibrary.Conv_VectorToLinearColor` (`SceneComponent.K2_GetComponentScale` _slicingcube)))
  (if (`|EnumEquality` SicingType _slicingtype)
    (if _inverted
      (bind _result (`/Engine/EditorBlueprintResources/StandardMacros.NegateFloat` SlicingOffset)
        (:`  `
          _)))
    (switch `ESlicingType` _slicingtype
      (:`X`
        (bind _returnvalue_3 (select `bool` _inverted :`false` SlicingOffset :`true` _result))
        (`SceneComponent.K2_SetRelativeLocation` _slicingcube (`KismetMathLibrary.MakeVector` _returnvalue_3) false false)
        (`KismetMaterialLibrary.SetVectorParameterValue` "/Game/Materials/SlicingMaterials/MPC_DissolveArea.MPC_DissolveArea" "LocationX" _returnvalue)
        (`KismetMaterialLibrary.SetVectorParameterValue` "/Game/Materials/SlicingMaterials/MPC_DissolveArea.MPC_DissolveArea" "ScaleX" _returnvalue_2))
      (:`Y`
        (`SceneComponent.K2_SetRelativeLocation` _slicingcube (`KismetMathLibrary.MakeVector` 0.0 _returnvalue_3) false false)
        (`KismetMaterialLibrary.SetVectorParameterValue` "/Game/Materials/SlicingMaterials/MPC_DissolveArea.MPC_DissolveArea" "LocationY" _returnvalue)
        (`KismetMaterialLibrary.SetVectorParameterValue` "/Game/Materials/SlicingMaterials/MPC_DissolveArea.MPC_DissolveArea" "ScaleY" _returnvalue_2))
      (:`Z`
        (`SceneComponent.K2_SetRelativeLocation` _slicingcube (`KismetMathLibrary.MakeVector` 0.0 0.0 _returnvalue_3) false false)
        (`KismetMaterialLibrary.SetVectorParameterValue` "/Game/Materials/SlicingMaterials/MPC_DissolveArea.MPC_DissolveArea" "LocationZ" _returnvalue)
        (`KismetMaterialLibrary.SetVectorParameterValue` "/Game/Materials/SlicingMaterials/MPC_DissolveArea.MPC_DissolveArea" "ScaleZ" _returnvalue_2)))))

(fn `Reset`
  (bind _slicingtype (`self.SlicingType`))
  (if (`self.Inverted`)
    (`self.ToogleInvertSlicing` _slicingtype))
  (`SceneComponent.K2_SetRelativeLocation` (`self.SlicingCube`) (0.0 0.0 0.0) false false)
  (`self.UpdateDissolveArea` _slicingtype))

(fn `ToogleActiveSlicing`
  (params (bIsCameraSlicing :type Boolean))
  (bind _output_get (set `self.bIsActiveSlicing` (not bIsCameraSlicing)))
  (if _output_get
    (`self.K2_SetActorLocation` (stale _output_get_2))
    (else
      (bind _output_get_2 (set `self.ActivePosition` (`self.K2_GetActorLocation`)))
      (`self.K2_SetActorLocation` (`self.InactivePosition`))))
  (`self.UpdateDissolveArea` (`self.SlicingType`)))

(fn `ToogleInvertSlicing`
  (params (SlicingType :type "ESlicingType Enum" :default "X") (bIsInverted :type Boolean))
  (bind (_returnvalue_x _returnvalue_y _returnvalue_z) (`KismetMathLibrary.BreakVector` (`self.K2_GetActorLocation`)))
  (bind _slicingtype (`self.SlicingType`))
  (bind _slicingcube (`self.SlicingCube`))
  (bind (_relativelocation_x _relativelocation_y _relativelocation_z) (`KismetMathLibrary.BreakVector` (`SceneComponent.RelativeLocation` _slicingcube)))
  (bind _returnvalue (`KismetMathLibrary.Conv_VectorToLinearColor` (`SceneComponent.K2_GetComponentLocation` _slicingcube)))
  (bind _returnvalue_2 (`KismetMathLibrary.Conv_VectorToLinearColor` (`SceneComponent.K2_GetComponentScale` _slicingcube)))
  (if (`|EnumEquality` SlicingType _slicingtype)
    (set `self.Inverted` bIsInverted)
    (switch `ESlicingType` _slicingtype
      (:`X`
        (bind _result (`/Engine/EditorBlueprintResources/StandardMacros.NegateFloat` _returnvalue_x)
          (:`  `
            (`self.K2_SetActorLocation` (`KismetMathLibrary.MakeVector` _result))
            (bind _result_2 (`/Engine/EditorBlueprintResources/StandardMacros.NegateFloat` _relativelocation_x)
              (:`  `
                (`SceneComponent.K2_SetRelativeLocation` _slicingcube (`KismetMathLibrary.MakeVector` _result_2) false false)
                (`KismetMaterialLibrary.SetVectorParameterValue` "/Game/Materials/SlicingMaterials/MPC_DissolveArea.MPC_DissolveArea" "LocationX" _returnvalue)
                (`KismetMaterialLibrary.SetVectorParameterValue` "/Game/Materials/SlicingMaterials/MPC_DissolveArea.MPC_DissolveArea" "ScaleX" _returnvalue_2))))))
      (:`Y`
        (bind _result_3 (`/Engine/EditorBlueprintResources/StandardMacros.NegateFloat` _returnvalue_y)
          (:`  `
            (`self.K2_SetActorLocation` (`KismetMathLibrary.MakeVector` 0.0 _result_3))
            (bind _result_4 (`/Engine/EditorBlueprintResources/StandardMacros.NegateFloat` _relativelocation_y)
              (:`  `
                (`SceneComponent.K2_SetRelativeLocation` _slicingcube (`KismetMathLibrary.MakeVector` 0.0 _result_4) false false)
                (`KismetMaterialLibrary.SetVectorParameterValue` "/Game/Materials/SlicingMaterials/MPC_DissolveArea.MPC_DissolveArea" "LocationY" _returnvalue)
                (`KismetMaterialLibrary.SetVectorParameterValue` "/Game/Materials/SlicingMaterials/MPC_DissolveArea.MPC_DissolveArea" "ScaleY" _returnvalue_2))))))
      (:`Z`
        (bind _result_5 (`/Engine/EditorBlueprintResources/StandardMacros.NegateFloat` _returnvalue_z)
          (:`  `
            (`self.K2_SetActorLocation` (`KismetMathLibrary.MakeVector` 0.0 0.0 _result_5))
            (bind _result_6 (`/Engine/EditorBlueprintResources/StandardMacros.NegateFloat` _relativelocation_z)
              (:`  `
                (`SceneComponent.K2_SetRelativeLocation` _slicingcube (`KismetMathLibrary.MakeVector` 0.0 0.0 _result_6) false false)
                (`KismetMaterialLibrary.SetVectorParameterValue` "/Game/Materials/SlicingMaterials/MPC_DissolveArea.MPC_DissolveArea" "LocationZ" _returnvalue)
                (`KismetMaterialLibrary.SetVectorParameterValue` "/Game/Materials/SlicingMaterials/MPC_DissolveArea.MPC_DissolveArea" "ScaleZ" _returnvalue_2)))))))))

(fn `UpdateDissolveArea`
  (params (Selection :type "ESlicingType Enum" :default "X"))
  (bind _slicingcube (`self.SlicingCube`))
  (bind _returnvalue (`KismetMathLibrary.Conv_VectorToLinearColor` (`SceneComponent.K2_GetComponentLocation` _slicingcube)))
  (bind _returnvalue_2 (`KismetMathLibrary.Conv_VectorToLinearColor` (`SceneComponent.K2_GetComponentScale` _slicingcube)))
  (switch `ESlicingType` Selection
    (:`X`
      (`KismetMaterialLibrary.SetVectorParameterValue` "/Game/Materials/SlicingMaterials/MPC_DissolveArea.MPC_DissolveArea" "LocationX" _returnvalue)
      (`KismetMaterialLibrary.SetVectorParameterValue` "/Game/Materials/SlicingMaterials/MPC_DissolveArea.MPC_DissolveArea" "ScaleX" _returnvalue_2))
    (:`Y`
      (`KismetMaterialLibrary.SetVectorParameterValue` "/Game/Materials/SlicingMaterials/MPC_DissolveArea.MPC_DissolveArea" "LocationY" _returnvalue)
      (`KismetMaterialLibrary.SetVectorParameterValue` "/Game/Materials/SlicingMaterials/MPC_DissolveArea.MPC_DissolveArea" "ScaleY" _returnvalue_2))
    (:`Z`
      (`KismetMaterialLibrary.SetVectorParameterValue` "/Game/Materials/SlicingMaterials/MPC_DissolveArea.MPC_DissolveArea" "LocationZ" _returnvalue)
      (`KismetMaterialLibrary.SetVectorParameterValue` "/Game/Materials/SlicingMaterials/MPC_DissolveArea.MPC_DissolveArea" "ScaleZ" _returnvalue_2))))

(fn `UserConstructionScript`)